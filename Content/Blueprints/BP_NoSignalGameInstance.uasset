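; Game instance for NoSignal that applies saved user settings at startup and manages level flow, pausing and player spawning.
; Scenes are streamed levels starting with MainMenu, with LoadLevel unloading the previous one and loading the next without blocking.
; Pause shows UI_Pause, while resume restores game input and clears the controller's CurrentUI.
; It spawns and possesses a single BP_Character, which quit-to-title destroys before clearing widgets and returning to MainMenu.
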(event Custom|Load%20Level
  (params (Level%20Name :type Name))
  ;[1 1 1] Level loading routine
  (bind _output_get (Variables|Default|SetLast%20Level%20Name (Variables|Default|GetLevel%20Name)))
  (bind _output_get_2 (Variables|Default|SetLevel%20Name Level%20Name))
  (Game|UnloadStreamLevel(byName) _output_get false)
  (Game|LoadStreamLevel(byName) _output_get_2 true))

(event Custom|On%20Initialize%20Scene
  ;[1 1 1] Initialize scene switch system & Open initial scene
  (bind _output_get (Variables|Default|SetLevel%20Name "MainMenu"))
  (Game|LoadStreamLevel(byName) _output_get true))

(event Custom|Quit%20To%20Title
  ;[1 1 1] Quit to title routine
  (Actor|DestroyActor (Variables|Default|GetPlayer%20Character))
  (Game|SetGamePaused false)
  (Viewport|RemoveAllWidgets)
  (bind _asbp_no_signal_player_controller (Utilities|Casting|CastToBP_NoSignalPlayerController (Game|GetPlayerController 0)))
  (Variables|/Game/Blueprints/BP_NoSignalPlayerController.BP_NoSignalPlayerController_C|SetCurrent%20UI _asbp_no_signal_player_controller 0)
  (CallFunction|LoadLevel "MainMenu"))

(event EventInit
  ;[1 0 0] Game Bootstrap (Load user settings & perform critical initializations)
  (bind _returnvalue (Settings|GetGameUserSettings))
  (Class|GameUserSettings|LoadSettings _returnvalue false)
  (Class|GameUserSettings|ApplySettings _returnvalue false))

(fn PauseGame
  (if (not (Game|IsGamePaused))
    (Game|SetGamePaused true)
    (bind _returnvalue (UserInterface|CreateWidget "/Game/UI/UI_Pause.UI_Pause_C"))
    (UserInterface|Viewport|AddtoViewport _returnvalue 0)))

(fn ResumeGame
  (bind _returnvalue (Game|GetPlayerController 0))
  (if (Game|IsGamePaused)
    (Game|SetGamePaused false)
    (Input|SetInputModeGameOnly _returnvalue false)
    (Variables|/Script/Engine.PlayerController|SetbShowMouseCursor _returnvalue false)
    (bind _asbp_no_signal_player_controller (Utilities|Casting|CastToBP_NoSignalPlayerController _returnvalue))
    (Widget|RemovefromParent (Variables|/Game/Blueprints/BP_NoSignalPlayerController.BP_NoSignalPlayerController_C|GetCurrent%20UI _asbp_no_signal_player_controller))
    (Variables|/Game/Blueprints/BP_NoSignalPlayerController.BP_NoSignalPlayerController_C|SetCurrent%20UI _asbp_no_signal_player_controller 0)))

(fn SpawnPlayer
  (params (Location :type Vector) (Rotation :type Rotator))
  (Utilities|IsValid (Variables|Default|GetPlayer%20Character)
    (:Is%20Not%20Valid
      (bind _returnvalue (Game|SpawnActorfromClass "/Game/Blueprints/Character/BP_Character.BP_Character_C" (Math|Transform|MakeTransform Location Rotation) "Undefined" 0 0))
      (bind _output_get (Variables|Default|SetPlayer%20Character _returnvalue))
      (Pawn|Possess (Game|GetPlayerController 0) _output_get))))
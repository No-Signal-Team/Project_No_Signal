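; BP_LightManager is a manager Blueprint that appears intended to track how many lights reach the player.
; BeginPlay caches all Light actors, and every Tick line-traces on Visibility from each to PlayerLocation, which this file never sets.
; An if/else-if macro adjusts NbLightSource from the trace result and a Lights.Contains check.
; Each element comes from Lights, so the increment never fires and every missed trace decrements the count.
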(event EventBeginPlay
  (bind _outactors (Actor|GetAllActorsOfClass "/Script/Engine.Light"))
  (Variables|Default|SetLights _outactors)
  (Development|PrintString "Hello"))

(event Collision|EventActorBeginOverlap
  (params (OtherActor :type Actor%20Object%20Reference)))

(event EventTick
  (params (DeltaSeconds :type Float%20%28single-precision%29))
  (bind _lights (Variables|Default|GetLights))
  (bind _nblightsource (Variables|Default|GetNbLightSource))
  (for _array_element _lights
    (bind _bhit (CallFunction|RaycasttoPlayer _array_element))
    (Utilities|IfElseifBranch (and (not (Utilities|Array|ContainsItem _lights _array_element)) _bhit) (and (Utilities|Array|ContainsItem _lights _array_element) (not _bhit))
      (:If%20Cond%201
        (Math|Integer|IncrementInt _nblightsource))
      (:Else%20If%20Cond%202
        (Math|Integer|DecrementInt _nblightsource)))))

(fn ConstructionScript)

(fn RaycasttoPlayer
  (params (Actor :type Actor%20Object%20Reference))
  (bind (_outhit _returnvalue) (Collision|LineTraceByChannel (Transformation|GetActorLocation Actor) (Variables|Default|GetPlayerLocation) "TraceTypeQuery1" false 0 "None"))
  (return _outhit _returnvalue))
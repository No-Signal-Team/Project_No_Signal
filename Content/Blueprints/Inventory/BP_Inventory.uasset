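; Inventory Blueprint that stores the player's items under a maximum weight limit and also holds a simple additive Health value.
; PickUpItem sphere-traces from the character camera, with debug drawing, and passes any BP_ParentItem hit to AddItem.
; AddItem checks weight, stacks stackable items by name, then destroys the world actor.
; RemoveItem decrements or deletes entries and recomputes weight; both refresh the inventory widget.
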(fn ConstructionScript)

(fn PickUpItem
  (bind _asbp_character (Utilities|Casting|CastToBP_Character (Game|GetPlayerCharacter 0)))
  (bind (_outhit _returnvalue) (Collision|SphereTraceByChannel (Transformation|GetWorldLocation (Variables|/Script/NoSignal.CharacterBase|GetcameraComponent _asbp_character)) (+ (Transformation|GetWorldLocation (Variables|/Script/NoSignal.CharacterBase|GetcameraComponent _asbp_character)) (* (Math|Vector|GetForwardVector (Variables|/Script/NoSignal.CharacterBase|GetcameraComponent _asbp_character)) "500.000000,500.000000,500.000000")) 5e+01 "TraceTypeQuery1" false 0 "ForDuration" true "(R=1.000000,G=0.000000,B=0.000000,A=1.000000)" "(R=0.000000,G=1.000000,B=0.000000,A=1.000000)" 2.0))
  (if _returnvalue
    (bind _asbp_parent_item (Utilities|Casting|CastToBP_ParentItem (.HitActor (Collision|BreakHitResult _outhit))))
    (CallFunction|AddItem _asbp_parent_item)))

(fn AddItem
  (params (itemRef :type BP%20Parent%20Item%20Object%20Reference))
  (bind _output_get (LocalVariables|SetitemStrucRef_ (Variables|/Game/Blueprints/Inventory/Items/BP_ParentItem.BP_ParentItem_C|Gets_items itemRef)))
  (LocalVariables|SetweightItemRef (.weight (Utilities|Struct|BreakS_Items _output_get)))
  (bind _isweightgood_ (CallFunction|CheckInventoryWeight (LocalVariables|GetweightItemRef)))
  (if _isweightgood_
    (if (.isStackable (Utilities|Struct|BreakS_Items _output_get))
      (if (!= (.Array%20Index (CallFunction|FindItembyName (Utilities|Struct|BreakS_Items _output_get))) -1)
        (Utilities|Array|SetArrayElem (Variables|Default|Getinventory) (.Array%20Index (CallFunction|FindItembyName (Utilities|Struct|BreakS_Items _output_get))) (Utilities|Struct|MakeS_Items (.name (Utilities|Struct|BreakS_Items (.Array%20Element (CallFunction|FindItembyName (Utilities|Struct|BreakS_Items _output_get))))) (.description (Utilities|Struct|BreakS_Items (.Array%20Element (CallFunction|FindItembyName (Utilities|Struct|BreakS_Items _output_get))))) (.icon (Utilities|Struct|BreakS_Items (.Array%20Element (CallFunction|FindItembyName (Utilities|Struct|BreakS_Items _output_get))))) (.isStackable (Utilities|Struct|BreakS_Items (.Array%20Element (CallFunction|FindItembyName (Utilities|Struct|BreakS_Items _output_get))))) (.type (Utilities|Struct|BreakS_Items (.Array%20Element (CallFunction|FindItembyName (Utilities|Struct|BreakS_Items _output_get))))) (.weight (Utilities|Struct|BreakS_Items (.Array%20Element (CallFunction|FindItembyName (Utilities|Struct|BreakS_Items _output_get))))) (+ (.numberItem (Utilities|Struct|BreakS_Items (.Array%20Element (CallFunction|FindItembyName (Utilities|Struct|BreakS_Items _output_get))))) 1) (.bonus (Utilities|Struct|BreakS_Items (.Array%20Element (CallFunction|FindItembyName (Utilities|Struct|BreakS_Items _output_get))))) (.itemClass (Utilities|Struct|BreakS_Items (.Array%20Element (CallFunction|FindItembyName (Utilities|Struct|BreakS_Items _output_get)))))))
        (CallFunction|SetInventoryWeight (LocalVariables|GetweightItemRef))
        (else
          (CallFunction|SetInventoryWeight (LocalVariables|GetweightItemRef) :!label _label)
          (Utilities|Array|Add (Variables|Default|Getinventory) (Variables|/Game/Blueprints/Inventory/Items/BP_ParentItem.BP_ParentItem_C|Gets_items itemRef))))
      (else
        (goto _label)))
    (Actor|DestroyActor itemRef)
    (Default|UpdateItemList (Variables|Default|GetWB_InventoryRef) (Variables|Default|Getinventory))))

(fn HealthManager
  (params (lifePoint :type Integer))
  (Variables|Default|Sethealth (+ lifePoint (Variables|Default|Gethealth))))

(fn CheckInventoryWeight
  (params (weight_Item :type Float%20%28double-precision%29))
  (return (<= (+ weight_Item (Variables|Default|GetinventoryWeight)) (Variables|Default|GetinventoryWeightMax))))

(fn SetInventoryWeight
  (params (weight_Item :type Float%20%28double-precision%29))
  (Variables|Default|SetinventoryWeight (+ weight_Item (Variables|Default|GetinventoryWeight))))

(fn UpdateInventoryWeight
  (Variables|Default|SetinventoryWeight 0.0)
  (for _array_element (Variables|Default|Getinventory)
    (Variables|Default|SetinventoryWeight (+ (* (.numberItem (Utilities|Struct|BreakS_Items _array_element)) (.weight (Utilities|Struct|BreakS_Items _array_element))) (Variables|Default|GetinventoryWeight)))))

(fn RemoveItem
  (params (Item :type S%20Items%20Structure))
  (bind _numberitem (Utilities|Struct|BreakS_Items Item))
  (bind _name (Utilities|Struct|BreakS_Items Item))
  (bind _array_index (CallFunction|FindItembyName _name))
  (bind _returnvalue (- _numberitem 1))
  (if (.isStackable (Utilities|Struct|BreakS_Items Item))
    (if (!= _returnvalue 0)
      (bind _structout (Utilities|Struct|SetmembersinS_Items Item _returnvalue))
      (Utilities|Array|SetArrayElem (Variables|Default|Getinventory) _array_index _structout)
      (else
        (Utilities|Array|RemoveIndex (Variables|Default|Getinventory) _array_index :!label _label)))
    (else
      (goto _label)))
  (Default|UpdateItemList (Variables|Default|GetWB_InventoryRef) (Variables|Default|Getinventory))
  (CallFunction|UpdateInventoryWeight)
  (return))

(fn FindItembyName
  (params (Name :type String))
  (bind (_array_element _array_index) (Utilities|Array|ForEachLoopwithBreak (Variables|Default|Getinventory))
    (:LoopBody
      (if (Utilities|Enum|Equal(Enum) (Utilities|Struct|BreakS_Items _array_element) Name)
        (return _array_element _array_index)))
    (:Completed
      (return "" -1))))
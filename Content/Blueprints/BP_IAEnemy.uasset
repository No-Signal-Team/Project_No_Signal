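; BP_IAEnemy is an AI enemy that wanders at random through the level.
; On BeginPlay, Walk moves it to a random reachable point around its current location and calls itself again on success; a failed move ends the loop.
; The perception update event and HandleSoundSense are empty stubs, and an unconnected branch holds an unfinished move and delayed return to Walk.
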(event OnTargetPerceptionUpdated(AIPerception)
  (params (Actor :type Actor%20Object%20Reference) (Stimulus :type AI%20Stimulus%20Structure)))

(event Custom|Walk
  (AI|AIMoveTo self (.RandomLocation (AI|Navigation|GetRandomReachablePointinRadius (Transformation|GetActorLocation) 1.5e+03 0 0)) 0 5.0 false
    (:OnSuccess
      (CallFunction|Walk))))

(event EventBeginPlay
  (CallFunction|Walk))

(fn ConstructionScript)

(fn HandleSoundSense)
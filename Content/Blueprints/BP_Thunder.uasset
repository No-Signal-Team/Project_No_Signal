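; BP_Thunder is a lightning effect that strikes repeatedly at random intervals of a few seconds from BeginPlay.
; Strike plays a timeline that drives the Y and emission material parameters on ThunderPlane.
; Shortly after each strike starts, the loop briefly overrides PPVolume's exposure compensation with manual metering for a screen flash, then reapplies the saved value, still in manual metering.
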(event Custom|Strike
  (bind _thunder_plane (Variables|Default|GetThunder_plane))
  (bind _thunder_strike (Timeline|Thunder_timeline PlayFromStart)
    (:Update
      (Rendering|Material|SetScalarParameterValueonMaterials _thunder_plane "Y" _thunder_strike)
      (Rendering|Material|SetScalarParameterValueonMaterials _thunder_plane "emission" (* (+ _thunder_strike 1.0) 3e+03)))))

(event EventBeginPlay
  (bind _pp_volume (Variables|Default|GetPP_Volume))
  (Utilities|FlowControl|Delay (Math|Random|RandomFloatinRange 3.0 1e+01) :!label _label)
  (CallFunction|Strike)
  (Utilities|FlowControl|Delay 0.2)
  (bind _output_get (Variables|Default|SetOriginal%20Exposure%20Compensation (Utilities|Struct|BreakPostProcessSettings (Variables|/Script/Engine.PostProcessVolume|GetSettings _pp_volume))))
  (Variables|/Script/Engine.PostProcessVolume|SetSettings _pp_volume (Utilities|Struct|MakePostProcessSettings "AEM_Manual" 12.0))
  (Utilities|FlowControl|Delay 0.1)
  (Variables|/Script/Engine.PostProcessVolume|SetSettings _pp_volume (Utilities|Struct|MakePostProcessSettings "AEM_Manual" _output_get))
  (goto _label))

(event Collision|EventActorBeginOverlap
  (params (OtherActor :type Actor%20Object%20Reference)))

(event EventTick
  (params (DeltaSeconds :type Float%20%28single-precision%29)))

(fn ConstructionScript)
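; Player character Blueprint that makes breathing audio respond to stress and handles pause input.
; Every tick, it copies StressAmount from its StressInfluencedEntityComponent into the "Stress" float parameter of the Breathing sound.
; Releasing the Pause input casts the game instance to BP_NoSignalGameInstance and calls PauseGame.
; An IfElseIfBranch macro provides three-way branching but is not used in the graphs shown.
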(event EventBeginPlay)

(event EventTick
  (params (DeltaSeconds :type Float%20%28single-precision%29))
  (CallFunction|UpdateStressSoundParameters))

(event Input|ActionEvents|InputActionPause
  (params (Key :type Key%20Structure))
  (:Released
    (bind _asbp_no_signal_game_instance (Utilities|Casting|CastToBP_NoSignalGameInstance (Game|GetGameInstance)))
    (Default|PauseGame _asbp_no_signal_game_instance)))

(fn ConstructionScript)

(fn UpdateStressSoundParameters
  (Audio|Parameter|SetFloatParameter (Variables|Default|GetBreathing) "Stress" (Variables|/Script/NoSignal.NS_StressInfluencedEntity|GetStressAmount (Variables|Default|GetStressInfluencedEntityComponent)) :!class /Script/AudioExtensions.AudioParameterControllerInterface))
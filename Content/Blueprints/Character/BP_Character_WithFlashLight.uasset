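; Player character Blueprint that carries a toggleable flashlight.
; On BeginPlay it spawns a BP_FlashLight actor at the mesh's SNFrontalLight socket and attaches it there.
; Each Tick it sets the light's rotation to the camera's, so the beam follows the view rather than the socket.
; The Toggle Light input flips the light's visibility and plays a switch sound at the socket.
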(event EventBeginPlay
  (bind _returnvalue (Game|SpawnActorfromClass "/Game/Blueprints/BP_FlashLight.BP_FlashLight_C" (Transformation|GetSocketTransform (Variables|Character|GetMesh) (Variables|Default|GetSN_FrontalLight) "RTS_World") "Undefined" 0 0))
  (bind _output_get (Variables|Default|SetSpotLight _returnvalue))
  (Transformation|AttachComponentToComponent _output_get (Variables|Character|GetMesh) (Variables|Default|GetSN_FrontalLight) "KeepWorld" "KeepRelative" "KeepRelative" true))

(event Collision|EventActorBeginOverlap
  (params (OtherActor :type Actor%20Object%20Reference)))

(event EventTick
  (params (DeltaSeconds :type Float%20%28single-precision%29))
  (Transformation|SetActorRotation (Variables|Default|GetSpotLight) (Transformation|GetWorldRotation (Variables|Default|GetcameraComponent))))

(event Input|ActionEvents|InputActionToggleLight
  (params (Key :type Key%20Structure :default "None"))
  ;[1 1 1] FlashLight Component Management
  (:Pressed
    (Rendering|ToggleVisibility (Variables|/Script/Engine.Actor|GetRootComponent (Variables|Default|GetSpotLight)) true)
    (Audio|PlaySoundatLocation (Variables|Default|GetS_LightToggle) (Transformation|GetSocketLocation (Variables|Character|GetMesh) (Variables|Default|GetSN_FrontalLight)) "0, 0, 0" 1.0 1.0 0.0 0 0 0 0)))

(fn ConstructionScript)
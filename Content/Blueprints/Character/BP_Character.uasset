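; Player character Blueprint that sets up and drives the player's flashlight, inventory, HUD and stress-based breathing audio.
; BeginPlay spawns a flashlight actor on a mesh socket and an inventory actor with its widget, and adds the HUD.
; Tick aligns the flashlight with the camera and feeds the stress component's value to the breathing sound.
; Input toggles the light, picks up items, switches the inventory with cursor and input lock, and calls game-instance pause or end-game.
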(event EventBeginPlay
  (CallFunction|CreateFrontalLight)
  ;[1 1 1] Create Inventory
  (bind _returnvalue (Game|SpawnActorfromClass "/Game/Blueprints/BP_Inventory.BP_Inventory_C" (Math|Conversions|ToTransform(Vector) "0, 0, 0") "Undefined" 0 0))
  (Variables|Default|SetInventory _returnvalue)
  (bind _returnvalue_2 (UserInterface|CreateWidget "/Game/Blueprints/Inventory/UI/WB_Inventory.WB_Inventory_C"))
  (Variables|/Game/Blueprints/BP_Inventory.BP_Inventory_C|SetWB_InventoryRef (Variables|Default|GetInventory) _returnvalue_2)
  (bind _returnvalue_3 (UserInterface|CreateWidget "/Game/UI/HUD/HUD.HUD_C" (Game|GetPlayerController 0)))
  (UserInterface|Viewport|AddtoViewport _returnvalue_3 0))

(event EventDestroyed
  (Actor|DestroyActor (Variables|Default|GetSpotLight)))

(event EventTick
  (params (DeltaSeconds :type Float%20%28single-precision%29))
  (CallFunction|RotateFrontalLight)
  (CallFunction|UpdateStressSoundParameters))

(event Input|ActionEvents|InputActionInterract
  (params (Key :type Key%20Structure :default "None"))
  ;[1 1 1] Interract with item
  (:Pressed
    (Default|PickUpItem (Variables|Default|GetInventory))))

(event Input|ActionEvents|InputActionInventory
  (params (Key :type Key%20Structure :default "None"))
  (bind _returnvalue (Game|GetPlayerController 0))
  (bind _returnvalue_2 (Game|GetPlayerController 0))
  (bind _inventory (Variables|Default|GetInventory))
  (bind _wb_inventoryref (Variables|/Game/Blueprints/BP_Inventory.BP_Inventory_C|GetWB_InventoryRef _inventory))
  ;[1 1 1] Open/Close Inventory
  (:Pressed
    (Utilities|IsValid (Variables|Default|GetInventory)
      (:Is%20Valid
        (Utilities|FlowControl|FlipFlop
          (:A
            (Widget|RemovefromParent _wb_inventoryref)
            (Variables|/Script/Engine.PlayerController|SetbShowMouseCursor _returnvalue_2 false)
            (Input|SetIgnoreMoveInput _returnvalue_2 false)
            (Input|SetIgnoreLookInput _returnvalue_2 false))
          (:B
            (UserInterface|Viewport|AddtoViewport _wb_inventoryref 0)
            (Default|LoadInventory (Variables|Default|GetInventory))
            (Variables|/Script/Engine.PlayerController|SetbShowMouseCursor _returnvalue true)
            (Input|SetIgnoreMoveInput _returnvalue true)
            (Input|SetIgnoreLookInput _returnvalue true)))))))

(event Input|ActionEvents|InputActionToggleLight
  (params (Key :type Key%20Structure :default "None"))
  ;[1 1 1] FlashLight Component Management
  (:Pressed
    (Rendering|ToggleVisibility (Variables|/Script/Engine.Actor|GetRootComponent (Variables|Default|GetSpotLight)) true)
    (Audio|PlaySoundatLocation (Variables|Default|GetFlashlightTickSound) (Transformation|GetSocketLocation (Variables|Character|GetMesh) (Variables|Default|GetSN_FrontalLight)) "0, 0, 0" 1.0 1.0 0.0 0 0 0 0)))

(event Input|ActionEvents|InputActionKys
  (params (Key :type Key%20Structure :default "None"))
  (:Pressed
    (bind _asbp_no_signal_game_instance (Utilities|Casting|CastToBP_NoSignalGameInstance (Game|GetGameInstance)))
    (Default|EndGame _asbp_no_signal_game_instance)))

(event Input|ActionEvents|InputActionPause
  (params (Key :type Key%20Structure :default "None"))
  (:Released
    (bind _asbp_no_signal_game_instance (Utilities|Casting|CastToBP_NoSignalGameInstance (Game|GetGameInstance)))
    (Default|PauseGame _asbp_no_signal_game_instance)))

(fn ConstructionScript)

(fn CreateFrontalLight
  (bind _returnvalue (Game|SpawnActorfromClass "/Game/Blueprints/BP_FlashLight.BP_FlashLight_C" (Transformation|GetSocketTransform (Variables|Character|GetMesh) (Variables|Default|GetSN_FrontalLight) "RTS_World") "Undefined" 0 0))
  (bind _output_get (Variables|Default|SetSpotLight _returnvalue))
  (Transformation|AttachComponentToComponent _output_get (Variables|Character|GetMesh) (Variables|Default|GetSN_FrontalLight) "KeepWorld" "KeepRelative" "KeepRelative" true))

(fn UpdateStressSoundParameters
  (Audio|Parameter|SetFloatParameter (Variables|Default|GetBreathing) "Stress" (Variables|/Script/NoSignal.NS_StressInfluencedEntity|GetStressAmount (Variables|Default|GetStressInfluencedEntityComponent)) :!class /Script/AudioExtensions.AudioParameterControllerInterface))

(fn RotateFrontalLight
  (Transformation|SetActorRotation (Variables|Default|GetSpotLight) (Transformation|GetWorldRotation (Variables|Default|GetcameraComponent))))
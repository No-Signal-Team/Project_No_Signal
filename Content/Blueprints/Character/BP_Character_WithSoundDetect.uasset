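; Character Blueprint that detects noises within a view cone through a PawnSensing component.
; On hearing a noise, it compares the angle between the camera's forward vector and the direction to the noise against the sensor's peripheral vision angle.
; Noises inside that cone only have their location printed as debug output.
; An inverse-square volume falloff calculation is present but unused.
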(event OnHearNoise(PawnSensing)
  (params (Instigator :type Pawn%20Object%20Reference) (Location :type Vector%20%28by%20ref%29 :default "0, 0, 0") (Volume :type Float%20%28single-precision%29))
  (bind _cameracomponent (Variables|Default|GetcameraComponent))
  (if (<= (Class|KismetMathLibrary|DegAcos (Math|Vector|DotProduct (Math|Vector|Normalize (- Location (Transformation|GetWorldLocation _cameracomponent))) (Math|Vector|Normalize (Math|Vector|GetForwardVector _cameracomponent)))) (Variables|/Script/AIModule.PawnSensingComponent|GetPeripheralVisionAngle (Variables|Default|GetPawnSensing)))
    (Development|PrintString (Utilities|String|ToString(Vector) Location))))

(event EventBeginPlay
  (|CallParentFunction) ; This node is disabled and will not be called.\nDrag off pins to build functionality.
)

(event Collision|EventActorBeginOverlap
  (params (OtherActor :type Actor%20Object%20Reference)))

(event EventTick
  (params (DeltaSeconds :type Float%20%28single-precision%29))
  (|CallParentFunction DeltaSeconds) ; This node is disabled and will not be called.\nDrag off pins to build functionality.
)

(fn ConstructionScript
  (|CallParentFunction))